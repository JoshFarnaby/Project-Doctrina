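; BP_Diegtic_Puzzle is a puzzle trigger actor that opens a numbered puzzle when the player enters its check volume.
; If creation is allowed, overlap adds WBP_Puzzle_Main to the viewport with its number and a self reference, switches to UI-only input and pauses the game.
; BeginPlay hides the in-world widget and removes the door for puzzle five.
; The diegetic widget and camera-possession path is present but never runs.
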(event OnComponentBeginOverlap(PuzzleCheck)
  (params (OverlappedComponent :type Primitive%20Component%20Object%20Reference) (OtherActor :type Actor%20Object%20Reference) (OtherComp :type Primitive%20Component%20Object%20Reference) (OtherBodyIndex :type Integer) (bFromSweep :type Boolean) (SweepResult :type Hit%20Result%20Structure%20%28by%20ref%29))
  (bind _returnvalue (Game|GetPlayerController 0))
  ;[1 0 0] On overlap with Puzzle Check, check for player and if true, create Main Puzzle Widget at relevent Puzzle Number.
  (if (Variables|Default|GetCan%20Create%20Puzzle?)
    (if (== OtherActor (Game|GetPlayerCharacter 0))
      (bind _returnvalue_2 (UserInterface|CreateWidget "/Game/Blueprints/UI/Widgets/WBP_Puzzle_Main.WBP_Puzzle_Main_C" 0 (Variables|Default|GetPuzzle%20Number) self))
      (UserInterface|Viewport|AddtoViewport _returnvalue_2 0)
      (Variables|/Script/Engine.PlayerController|SetbShowMouseCursor _returnvalue true)
      (Input|SetInputModeUIOnly _returnvalue _returnvalue_2 "LockInFullscreen" true)
      (Game|SetGamePaused true))))

(event EventBeginPlay
  ;[0 0.05329 1] Set visibility of Puzzle Widget and Puzzle Door on Begin Play to hidden.
  (Rendering|SetVisibility (Variables|Default|GetPuzzle%20Widget) false false)
  (if (== (Variables|Default|GetPuzzle%20Number) 5)
    (Components|DestroyComponent (Variables|Default|GetSM_Puzzle_Door))))

(fn ConstructionScript)