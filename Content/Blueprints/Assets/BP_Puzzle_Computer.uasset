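; Puzzle computer actor with a linked door that stays locked until its puzzle is completed.
; Player overlap with PuzzleCheck, gated by CanCreatePuzzle, shows an interact widget and passes the puzzle number and actor to the player controller.
; A second trigger shows a fading door-locked widget.
; PuzzleComplete teleports the door to an arrow, turns the light green and destroys that trigger; puzzle 10 removes its door frame on BeginPlay.
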(event OnComponentBeginOverlap(PuzzleCheck)
  (params (OverlappedComponent :type Primitive%20Component%20Object%20Reference) (OtherActor :type Actor%20Object%20Reference) (OtherComp :type Primitive%20Component%20Object%20Reference) (OtherBodyIndex :type Integer) (bFromSweep :type Boolean) (SweepResult :type Hit%20Result%20Structure%20%28by%20ref%29))
  ;[1 0 0] On overlap with Puzzle Check, check for player and if true, create Interact Widget.
  (if (Variables|Default|GetCan%20Create%20Puzzle?)
    (if (== OtherActor (Game|GetPlayerCharacter 0))
      (bind _returnvalue (UserInterface|CreateWidget "/Game/Blueprints/UI/Widgets/WBP_Interact.WBP_Interact_C"))
      (UserInterface|Viewport|AddtoViewport _returnvalue 0)
      (Class|BPIUI|Interact(Message) (Game|GetPlayerController 0) true (Variables|Default|GetPuzzle%20Number) self))))

(event OnComponentEndOverlap(PuzzleCheck)
  (params (OverlappedComponent :type Primitive%20Component%20Object%20Reference) (OtherActor :type Actor%20Object%20Reference) (OtherComp :type Primitive%20Component%20Object%20Reference) (OtherBodyIndex :type Integer))
  ;[1 0 0] Remove Interact Widget On Compoenent End Overlap on Puzzle Check.
  (if (Variables|Default|GetCan%20Create%20Puzzle?)
    (if (== OtherActor (Game|GetPlayerCharacter 0))
      (Class|BPIUI|Interact(Message) (Game|GetPlayerController 0) false (Variables|Default|GetPuzzle%20Number) self)
      (bind _foundwidgets (Widget|GetAllWidgetsOfClass "/Game/Blueprints/UI/Widgets/WBP_Interact.WBP_Interact_C" true))
      (for _array_element _foundwidgets
        (Class|UserWidget|PlayAnimationReverse _array_element (Variables|/Game/Blueprints/UI/Widgets/WBP_Interact.WBP_Interact_C|GetFade _array_element) 1.0 false)
        (Utilities|FlowControl|Delay (Class|WidgetAnimation|GetEndTime (Variables|/Game/Blueprints/UI/Widgets/WBP_Interact.WBP_Interact_C|GetFade _array_element)))
        (Widget|RemovefromParent _array_element)))))

(event OnComponentBeginOverlap(PuzzleDoorCheck)
  (params (OverlappedComponent :type Primitive%20Component%20Object%20Reference) (OtherActor :type Actor%20Object%20Reference) (OtherComp :type Primitive%20Component%20Object%20Reference) (OtherBodyIndex :type Integer) (bFromSweep :type Boolean) (SweepResult :type Hit%20Result%20Structure%20%28by%20ref%29))
  ;[1 0 0] Create Puzzle Door Locked on Puzzle Door Check begin overlap.
  (if (== OtherActor (Game|GetPlayerCharacter 0))
    (bind _returnvalue (UserInterface|CreateWidget "/Game/Blueprints/UI/Widgets/WBP_Puzzle_Door_Locked.WBP_Puzzle_Door_Locked_C"))
    (UserInterface|Viewport|AddtoViewport _returnvalue 0)))

(event OnComponentEndOverlap(PuzzleDoorCheck)
  (params (OverlappedComponent :type Primitive%20Component%20Object%20Reference) (OtherActor :type Actor%20Object%20Reference) (OtherComp :type Primitive%20Component%20Object%20Reference) (OtherBodyIndex :type Integer))
  ;[1 0 0] Play Fade in reverse and remove Puzzle Door Locked from parent on Puzzle Door Check end overlap.
  (if (== OtherActor (Game|GetPlayerCharacter 0))
    (Utilities|FlowControl|DelayUntilNextTick)
    (Class|UserWidget|PlayAnimationReverse (stale OnComponentBeginOverlap(PuzzleDoorCheck) _returnvalue) (Variables|/Game/Blueprints/UI/Widgets/WBP_Puzzle_Door_Locked.WBP_Puzzle_Door_Locked_C|GetFade (stale OnComponentBeginOverlap(PuzzleDoorCheck) _returnvalue)) 1.0 false)
    (Utilities|FlowControl|Delay (Class|WidgetAnimation|GetEndTime (Variables|/Game/Blueprints/UI/Widgets/WBP_Puzzle_Door_Locked.WBP_Puzzle_Door_Locked_C|GetFade (stale OnComponentBeginOverlap(PuzzleDoorCheck) _returnvalue))))
    (Widget|RemovefromParent (stale OnComponentBeginOverlap(PuzzleDoorCheck) _returnvalue))))

(event Custom|Puzzle%20Complete
  ;[1 0 0] Set location of door to the arrow's world location,change puzzle light colour and destroy Puzzle Door Check on Puzzle Complete.
  (Transformation|SetWorldLocation (Variables|Default|GetSM_Puzzle_Door) (Transformation|GetWorldLocation (Variables|Default|GetArrow)) false false)
  (Rendering|Components|Light|SetLightColor (Variables|Default|GetPuzzle%20Light) "(R=0.000000,G=1.000000,B=0.277211,A=1.000000)" true)
  (Components|DestroyComponent (Variables|Default|GetPuzzle%20Door%20Check)))

(event EventBeginPlay
  ;[0 0.05329 1] Set visibility of Puzzle Widget and Puzzle Door on Begin Play to hidden.
  (Rendering|SetVisibility (Variables|Default|GetPuzzle%20Widget) false false)
  (if (== (Variables|Default|GetPuzzle%20Number) 10)
    (Components|DestroyComponent (Variables|Default|GetSM_Puzzle_Door_Frame))))

(fn ConstructionScript)

(fn Interact
  (params (Can%20be%20Interacted? :type Boolean) (Puzzle%20Number :type Byte :default 0) (Diegetic%20Puzzle%20Element%20 :type BP%20Puzzle%20Computer%20Object%20Reference)))