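; BP_Door_Locked is a door actor that shows a locked-door notice while the player character is inside its DoorCheck trigger.
; Begin overlap creates a WBP_Door_Locked widget and adds it to the viewport.
; End overlap waits a tick, plays the widget's Fade animation in reverse, then removes it after a delay matching the animation's end time.
; The file contains no unlock or door movement logic.
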(event OnComponentBeginOverlap(DoorCheck)
  (params (OverlappedComponent :type Primitive%20Component%20Object%20Reference) (OtherActor :type Actor%20Object%20Reference) (OtherComp :type Primitive%20Component%20Object%20Reference) (OtherBodyIndex :type Integer) (bFromSweep :type Boolean) (SweepResult :type Hit%20Result%20Structure%20%28by%20ref%29))
  ;[1 0 0] Create Door Locked on Door Check begin overlap.
  (if (== OtherActor (Game|GetPlayerCharacter 0))
    (bind _returnvalue (UserInterface|CreateWidget "/Game/Blueprints/UI/Widgets/WBP_Door_Locked.WBP_Door_Locked_C"))
    (UserInterface|Viewport|AddtoViewport _returnvalue 0)))

(event OnComponentEndOverlap(DoorCheck)
  (params (OverlappedComponent :type Primitive%20Component%20Object%20Reference) (OtherActor :type Actor%20Object%20Reference) (OtherComp :type Primitive%20Component%20Object%20Reference) (OtherBodyIndex :type Integer))
  ;[1 0 0] Play Fade in reverse and remove Door Locked from parent on Door Check end overlap.
  (if (== OtherActor (Game|GetPlayerCharacter 0))
    (Utilities|FlowControl|DelayUntilNextTick)
    (Class|UserWidget|PlayAnimationReverse (stale OnComponentBeginOverlap(DoorCheck) _returnvalue) (Variables|/Game/Blueprints/UI/Widgets/WBP_Door_Locked.WBP_Door_Locked_C|GetFade (stale OnComponentBeginOverlap(DoorCheck) _returnvalue)) 1.0 false)
    (Utilities|FlowControl|Delay (Class|WidgetAnimation|GetEndTime (Variables|/Game/Blueprints/UI/Widgets/WBP_Door_Locked.WBP_Door_Locked_C|GetFade (stale OnComponentBeginOverlap(DoorCheck) _returnvalue))))
    (Widget|RemovefromParent (stale OnComponentBeginOverlap(DoorCheck) _returnvalue))))

(fn ConstructionScript)