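; BP_Doctrina_Player_Controller handles input for the pause menu, puzzle interaction and tutorial playback.
; Pause input toggles WBP_Pause_Menu outside the main menu level, saving options and resuming play on close.
; An Interact event sets availability, letting interact input open WBP_Puzzle_Main for a puzzle number, pause the game and show the cursor.
; Tutorial input flip-flops the drag element's teaching animation forward or faster in reverse, except on first drag.
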(event Input|EnhancedActionEvents|EnhancedInputActionIA_Pause
  (params (ActionValue :type Boolean) (ElapsedSeconds :type Float%20%28double-precision%29) (TriggeredSeconds :type Float%20%28double-precision%29) (InputAction :type Input%20Action%20Object%20Reference :default "/Game/Blueprints/Input/Input_Actions/IA_Pause.IA_Pause"))
  ;[1 0 0] Create and remove pause menu on pause button started.
  (:Started
    (CallFunction|PauseMenu)))

(event Input|EnhancedActionEvents|EnhancedInputActionIA_Interact
  (params (ActionValue :type Vector%202D%20Structure) (ElapsedSeconds :type Float%20%28double-precision%29) (TriggeredSeconds :type Float%20%28double-precision%29) (InputAction :type Input%20Action%20Object%20Reference :default "/Game/Blueprints/Input/Input_Actions/IA_Interact.IA_Interact"))
  (bind _returnvalue (Game|GetPlayerController 0))
  ;[1 0 0] If can be interacted with, create Puzzle Main Widget at relevent Puzzle Number.
  (:Started
    (if (Variables|Default|GetCan%20Be%20Interacted?)
      (Variables|Default|SetCan%20Be%20Interacted? false)
      (bind _returnvalue_2 (UserInterface|CreateWidget "/Game/Blueprints/UI/Widgets/WBP_Puzzle_Main.WBP_Puzzle_Main_C" 0 (stale EventInteract Puzzle%20Number) (stale EventInteract Diegetic%20Puzzle%20Element%20)))
      (bind _output_get (Variables|Default|SetMain%20Puzzle%20Ref _returnvalue_2))
      (Variables|Default|SetDrag%20Element%20Ref (Variables|/Game/Blueprints/UI/Widgets/WBP_Puzzle_Main.WBP_Puzzle_Main_C|GetDrag%20Element%20Ref _output_get))
      (UserInterface|Viewport|AddtoViewport _returnvalue_2 0)
      (Variables|/Script/Engine.PlayerController|SetbShowMouseCursor _returnvalue true)
      (Input|SetInputModeGameandUI _returnvalue _output_get "LockInFullscreen" false true)
      (Game|SetGamePaused true))))

(event Input|EnhancedActionEvents|EnhancedInputActionIA_Tuitorial
  (params (ActionValue :type Vector%202D%20Structure) (ElapsedSeconds :type Float%20%28double-precision%29) (TriggeredSeconds :type Float%20%28double-precision%29) (InputAction :type Input%20Action%20Object%20Reference :default "/Game/Blueprints/Input/Input_Actions/IA_Tuitorial.IA_Tuitorial"))
  ;[1 0 0] Play Tutorial in reverse and forwards on Tutorial Input.
  (:Started
    (bind _foundwidgets (Widget|GetAllWidgetsOfClass "/Game/Blueprints/UI/Widgets/WBP_Drag_Element.WBP_Drag_Element_C" false))
    (for _array_element _foundwidgets
      _)
    (if (not (Variables|/Game/Blueprints/UI/Widgets/WBP_Drag_Element.WBP_Drag_Element_C|GetIs%20First%20Drag? _array_element))
      (bind _foundwidgets_2 (Widget|GetAllWidgetsOfClass (Variables|/Game/Blueprints/UI/Widgets/WBP_Drag_Element.WBP_Drag_Element_C|GetTeaching%20Puzzle%20Design _array_element) false))
      (for _array_element_2 _foundwidgets_2
        _)
      (Utilities|FlowControl|FlipFlop
        (:A
          (Class|UserWidget|PlayAnimationForward _array_element_2 (Variables|/Game/Blueprints/UI/Widgets/WBP_Drag_Element.WBP_Drag_Element_C|GetAnimation _array_element) 1.0 false))
        (:B
          (Class|UserWidget|PlayAnimationReverse _array_element_2 (Variables|/Game/Blueprints/UI/Widgets/WBP_Drag_Element.WBP_Drag_Element_C|GetAnimation _array_element) 2.0 false))))))

(event EventPauseMenu
  (bind _returnvalue (Game|GetPlayerController 0))
  ;[0 0.006212 1] Create and remove pause menu on flip flop.
  (bind _returnvalue_2 (Game|GetCurrentLevelName true))
  (if (not (Utilities|Enum|Equal(Enum) _returnvalue_2 "L_Main_Menu"))
    (Utilities|FlowControl|FlipFlop
      (:A
        (bind _returnvalue_3 (UserInterface|CreateWidget "/Game/Blueprints/UI/Widgets/WBP_Pause_Menu.WBP_Pause_Menu_C"))
        (UserInterface|Viewport|AddtoViewport _returnvalue_3 0))
      (:B
        (Default|SaveOptions (Variables|/Game/Blueprints/UI/Widgets/WBP_Pause_Menu.WBP_Pause_Menu_C|GetOptionsMenu _returnvalue_3))
        (Widget|RemovefromParent _returnvalue_3)
        (Variables|/Script/Engine.PlayerController|SetbShowMouseCursor _returnvalue false)
        (Game|SetGamePaused false)
        (Input|SetInputModeGameOnly _returnvalue true)))))

(event EventInteract
  (params (Can%20be%20Interacted? :type Boolean) (Puzzle%20Number :type Byte :default 0) (Diegetic%20Puzzle%20Element%20 :type BP%20Diegtic%20Puzzle%20Object%20Reference))
  ;[1 0 0] When Event Interact is called, set relevent variables for IA-Interact.
  (Variables|Default|SetCan%20Be%20Interacted? Can%20be%20Interacted?))

(fn ConstructionScript)